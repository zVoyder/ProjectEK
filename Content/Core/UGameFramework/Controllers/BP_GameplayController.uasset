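; Gameplay controller that handles the character menu and inventory input for the player.
; On BeginPlay it creates the character menu widget, registers it with MenuManager by gameplay tag and binds its close event.
; Enhanced Input actions toggle the menu or forward item requests like drag-drop, equip, rotate, split and compare, with press/release pairs for held actions.
; OpenLootPanel and ClearLootPanel show and close a loot inventory inside that menu's inventory panel.
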(event EventBeginPlay
  (|CallParentFunction)
  (CallFunction|InitMenusGraph))

(event Custom|InitMenusGraph
  (bind _returnvalue (UserInterface|CreateWidget "/Game/Core/Features/UI/Menus/WBP_CharacterMenu.WBP_CharacterMenu_C" self))
  (Class|MenuManager|AddMenu (Variables|Default|GetMenuManager) "(TagName=\"UI.Menu.Character\")" _returnvalue 1)
  (EventDispatchers|AssignOnMenuClosed _returnvalue (EventDispatchers|CreateEvent :!event ClearLootPanel)))

(event Input|EnhancedActionEvents|EnhancedInputActionIA_EquipItem_0
  (params (ActionValue :type Boolean) (ElapsedSeconds :type Float%20%28double-precision%29) (TriggeredSeconds :type Float%20%28double-precision%29) (InputAction :type Input%20Action%20Object%20Reference :default "/Game/Core/Inputs/InputActions/Menus/IA_EquipItem_0.IA_EquipItem_0"))
  ;[1 0 0] Inventory Actions
  (Class|TetrisInventoriesUtility|RequestEquipUnequip))

(event Input|EnhancedActionEvents|EnhancedInputActionIA_EquipItem_1
  (params (ActionValue :type Boolean) (ElapsedSeconds :type Float%20%28double-precision%29) (TriggeredSeconds :type Float%20%28double-precision%29) (InputAction :type Input%20Action%20Object%20Reference :default "/Game/Core/Inputs/InputActions/Menus/IA_EquipItem_1.IA_EquipItem_1"))
  ;[1 0 0] Inventory Actions
  (Class|TetrisInventoriesUtility|RequestEquipUnequip 1))

(event Input|EnhancedActionEvents|EnhancedInputActionIA_RotateItem
  (params (ActionValue :type Boolean) (ElapsedSeconds :type Float%20%28double-precision%29) (TriggeredSeconds :type Float%20%28double-precision%29) (InputAction :type Input%20Action%20Object%20Reference :default "/Game/Core/Inputs/InputActions/Menus/IA_RotateItem.IA_RotateItem"))
  ;[1 0 0] Inventory Actions
  (Class|TetrisInventoriesUtility|RequestRotate))

(event Input|EnhancedActionEvents|EnhancedInputActionIA_SplitItem
  (params (ActionValue :type Boolean) (ElapsedSeconds :type Float%20%28double-precision%29) (TriggeredSeconds :type Float%20%28double-precision%29) (InputAction :type Input%20Action%20Object%20Reference :default "/Game/Core/Inputs/InputActions/Menus/IA_SplitItem.IA_SplitItem"))
  ;[1 0 0] Inventory Actions
  (:Started
    (Class|TetrisInventoriesUtility|RequestSplit))
  (:Completed
    (Class|TetrisInventoriesUtility|RequestCancelSplit)))

(event Input|EnhancedActionEvents|EnhancedInputActionIA_CompareItem
  (params (ActionValue :type Boolean) (ElapsedSeconds :type Float%20%28double-precision%29) (TriggeredSeconds :type Float%20%28double-precision%29) (InputAction :type Input%20Action%20Object%20Reference :default "/Game/Core/Inputs/InputActions/Menus/IA_CompareItem.IA_CompareItem"))
  ;[1 0 0] Inventory Actions
  (:Started
    (Class|RPGInventoriesUtility|RequestCompare true))
  (:Completed
    (Class|RPGInventoriesUtility|RequestCompare false)))

(event Input|EnhancedActionEvents|EnhancedInputActionIA_CharacterMenu
  (params (ActionValue :type Boolean) (ElapsedSeconds :type Float%20%28double-precision%29) (TriggeredSeconds :type Float%20%28double-precision%29) (InputAction :type Input%20Action%20Object%20Reference :default "/Game/Core/Inputs/InputActions/Menus/IA_CharacterMenu.IA_CharacterMenu"))
  ;[0.15 0.15 0.15 0.5] Menus Actions
  (Class|MenuManager|ToggleMenu (Variables|Default|GetMenuManager) "(TagName=\"UI.Menu.Character\")"))

(event Input|EnhancedActionEvents|EnhancedInputActionIA_DiscardItem
  (params (ActionValue :type Boolean) (ElapsedSeconds :type Float%20%28double-precision%29) (TriggeredSeconds :type Float%20%28double-precision%29) (InputAction :type Input%20Action%20Object%20Reference :default "/Game/Core/Inputs/InputActions/Menus/IA_DiscardItem.IA_DiscardItem"))
  ;[1 0 0] Inventory Actions
  (Class|TetrisInventoriesUtility|RequestDiscard))

(event Input|EnhancedActionEvents|EnhancedInputActionIA_DragDrop
  (params (ActionValue :type Boolean) (ElapsedSeconds :type Float%20%28double-precision%29) (TriggeredSeconds :type Float%20%28double-precision%29) (InputAction :type Input%20Action%20Object%20Reference :default "/Game/Core/Inputs/InputActions/Menus/IA_DragDrop.IA_DragDrop"))
  ;[1 0 0] Inventory Actions
  (:Started
    (Class|TetrisInventoriesUtility|RequestDrag))
  (:Completed
    (Class|TetrisInventoriesUtility|RequestDrop)))

(fn ConstructionScript)

(fn OpenLootPanel
  (params (RelatedInventory :type Tetris%20Inventory%20Object%20Reference) (LootName :type Text))
  (bind _returnvalue (Class|MenuManager|ToggleMenu (Variables|Default|GetMenuManager) "(TagName=\"UI.Menu.Character\")"))
  (bind _aswbp_character_menu (Utilities|Casting|CastToWBP_CharacterMenu _returnvalue))
  (Default|OpenLootInventory (Variables|/Game/Core/Features/UI/Menus/WBP_CharacterMenu.WBP_CharacterMenu_C|GetWBP_InventoryPanel _aswbp_character_menu) RelatedInventory LootName))

(fn ClearLootPanel
  (bind _aswbp_character_menu (Utilities|Casting|CastToWBP_CharacterMenu (Class|MenuManager|GetMenubyTag (Variables|Default|GetMenuManager) "(TagName=\"UI.Menu.Character\")")))
  (Default|CloseLootInventory (Variables|/Game/Core/Features/UI/Menus/WBP_CharacterMenu.WBP_CharacterMenu_C|GetWBP_InventoryPanel _aswbp_character_menu)))
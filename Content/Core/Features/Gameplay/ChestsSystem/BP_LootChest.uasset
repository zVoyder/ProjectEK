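; Loot chest that fills its RPG inventory with random gear, weapons, generic items and currency when first opened.
; Four generator functions roll counts from configured ranges, drawing entries from data maps; currency is always the Patronian Shield asset.
; Generic items reuse WeaponsRange for their roll count.
; Map keys and values use separate random index rolls, so an item's data and its generation settings or amount bounds can come from different entries.
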(event EventOnChestFirstOpen
  (CallFunction|GenerateGears)
  (CallFunction|GenerateWeapons)
  (CallFunction|GenerateItems)
  (CallFunction|GenerateCurrency))

(fn ConstructionScript
  (|CallParentFunction))

(fn GenerateGears
  (bind _gearsrange (Variables|Generation|GetGearsRange))
  (bind _gears (Variables|Generation|GetGears))
  (bind _returnvalue (Utilities|Map|Length _gears))
  (bind _returnvalue_2 (- _returnvalue 1))
  (bind _returnvalue_3 (Math|Random|RandomIntegerinRange 0 _returnvalue_2))
  (bind (_key _value) (Utilities|Map|GetKeyValueByIndex _gears _returnvalue_3))
  (if (Utilities|Map|IsNotEmpty (Variables|Generation|GetGears))
    (for _index (range 0 (- (Math|Random|RandomIntegerinRange (.value (.lowerbound _gearsrange)) (.value (.upperbound _gearsrange))) 1))
      (bind _returnvalue_4 (Class|RPGFactory|CreateRPGGearItemwithGenerationSet _key _value))
      (Class|InventoryBase|TryAddItem (Variables|Default|GetRPGInventory) _returnvalue_4))))

(fn GenerateWeapons
  (bind _weapons (Variables|Generation|GetWeapons))
  (bind _weaponsrange (Variables|Generation|GetWeaponsRange))
  (bind _returnvalue (Utilities|Map|Length _weapons))
  (bind _returnvalue_2 (- _returnvalue 1))
  (bind _returnvalue_3 (Math|Random|RandomIntegerinRange 0 _returnvalue_2))
  (bind (_key _value) (Utilities|Map|GetKeyValueByIndex _weapons _returnvalue_3))
  (if (Utilities|Map|IsNotEmpty (Variables|Generation|GetWeapons))
    (for _index (range 0 (- (Math|Random|RandomIntegerinRange (.value (.lowerbound _weaponsrange)) (.value (.upperbound _weaponsrange))) 1))
      (bind _returnvalue_4 (Class|RPGFactory|CreateRPGGearItem _key _value))
      (Class|InventoryBase|TryAddItem (Variables|Default|GetRPGInventory) _returnvalue_4))))

(fn GenerateItems
  (bind _generics (Variables|Generation|GetGenerics))
  (bind _weaponsrange (Variables|Generation|GetWeaponsRange))
  (bind _returnvalue (Utilities|Map|Length _generics))
  (bind _returnvalue_2 (- _returnvalue 1))
  (bind _returnvalue_3 (Math|Random|RandomIntegerinRange 0 _returnvalue_2))
  (bind (_key _value) (Utilities|Map|GetKeyValueByIndex _generics _returnvalue_3))
  (if (Utilities|Map|IsNotEmpty (Variables|Generation|GetGenerics))
    (for _index (range 0 (- (Math|Random|RandomIntegerinRange (.value (.lowerbound _weaponsrange)) (.value (.upperbound _weaponsrange))) 1))
      (Class|InventoryBase|AddNewItem (Variables|Default|GetRPGInventory) _key (Math|Random|RandomIntegerinRange (.value (.lowerbound _value)) (.value (.upperbound _value)))))))

(fn GenerateCurrency
  (bind _currencyrange (Variables|Generation|GetCurrencyRange))
  (Class|InventoryBase|AddNewItem (Variables|Default|GetRPGInventory) "/Game/Data/Inventory/Items/Generics/DA_PatronianShield.DA_PatronianShield" (Math|Random|RandomIntegerinRange (.value (.lowerbound _currencyrange)) (.value (.upperbound _currencyrange)))))
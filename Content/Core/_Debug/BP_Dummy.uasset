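; BP_Dummy is a debug target character for testing hit box damage, ragdolling and limb dismemberment.
; Its Dismemberer component initializes on the mesh at BeginPlay.
; Any damage reported by the HitBoxManager turns the mesh into a simulated ragdoll and disables capsule collision.
; Point damage with the BP_DismemberDamageType damage type also dismembers the hit bone's limb, passing the damage with zero impulse.
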(event OnHitBoxPointDamage(HitBoxManager)
  (params (BaseDamage :type Float%20%28single-precision%29) (TotalDamage :type Float%20%28single-precision%29) (HitLocation :type Vector :default "0, 0, 0") (HitNormal :type Vector :default "0, 0, 0") (BoneName :type Name :default "None") (DamageType :type Damage%20Type%20Object%20Reference) (InstigatedBy :type Controller%20Object%20Reference) (DamageCauser :type Actor%20Object%20Reference))
  (Class|KismetSystemLibrary|IsObjectOfSoftClass DamageType "/Game/Core/Features/Gameplay/WeaponSystem/DamageTypes/BP_DismemberDamageType.BP_DismemberDamageType_C"
    (:True
      (Class|Dismemberer|DismemberLimb (Variables|Default|GetDismemberer) BoneName "0, 0, 0" TotalDamage))))

(event OnHitBoxAnyDamage(HitBoxManager)
  (params (BaseDamage :type Float%20%28single-precision%29) (TotalDamage :type Float%20%28single-precision%29) (DamageType :type Damage%20Type%20Object%20Reference) (InstigatedBy :type Controller%20Object%20Reference) (DamageCauser :type Actor%20Object%20Reference))
  (Collision|SetCollisionProfileName (Variables|Character|GetMesh) "Ragdoll" true :!class /Script/Engine.PrimitiveComponent)
  (Physics|SetSimulatePhysics (Variables|Character|GetMesh) true)
  (Collision|SetCollisionEnabled (Variables|Collision|GetCapsuleComponent) "NoCollision"))

(event EventBeginPlay
  (Class|Dismemberer|Init (Variables|Default|GetDismemberer) (Variables|Character|GetMesh)))

(fn ConstructionScript)
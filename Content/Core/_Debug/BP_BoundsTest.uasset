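; Debug test actor that visualizes its bounds and snaps itself to the surface below it.
; On BeginPlay, SnapToGround line-traces on the Visibility channel along the actor's down vector and teleports it to the hit.
; The Z offset compensates for the pivot's position within the bounds, placing the bottom of the bounds at impact height.
; Every Tick draws a green debug box around the actor's bounds, including non-colliding components.
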(event EventBeginPlay
  (CallFunction|SnaptoGround))

(event EventTick
  (params (DeltaSeconds :type Float%20%28single-precision%29))
  (bind (_origin _boxextent) (Collision|GetActorBounds false false))
  (Rendering|Debug|DrawDebugBox _origin _boxextent "(R=0.000000,G=1.000000,B=0.000000,A=1.000000)" "0, 0, 0" 0.0 2.0))

(fn ConstructionScript)

(fn SnaptoGround
  (bind (_origin _boxextent) (Collision|GetActorBounds false false))
  (bind _returnvalue (Transformation|GetActorLocation))
  (bind (_outhit _returnvalue_2) (Collision|LineTraceByChannel _returnvalue (+ _returnvalue (* (Transformation|GetActorUpVector) 1e+07 -1.0)) "TraceTypeQuery1" false 0 "None"))
  (if _returnvalue_2
    (Transformation|SetActorLocation (Math|Vector|MakeVector (.X (Math|Vector|BreakVector (.ImpactPoint (Collision|BreakHitResult _outhit)))) (.Y (Math|Vector|BreakVector (.ImpactPoint (Collision|BreakHitResult _outhit)))) (+ (.Z (Math|Vector|BreakVector (.ImpactPoint (Collision|BreakHitResult _outhit)))) (- (.Z (Math|Vector|BreakVector _boxextent)) (- (.Z (Math|Vector|BreakVector _origin)) (.Z (Math|Vector|BreakVector (Transformation|GetActorLocation))))))) false true)))
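; Arrow projectile for the weapon system that leaves an arrow item drop where it hits.
; On hit it creates an item from the arrow data asset and drops it slightly forward along its facing by a random offset, then runs the parent hit logic.
; If the hit actor is a Pawn, the dropped item actor attaches to the hit component's bone, keeping its world location and rotation.
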(event EventOnProjectileHit
  (params (ImpactResult :type Hit%20Result%20Structure%20%28by%20ref%29) (ImpactVelocity :type Vector%20%28by%20ref%29 :default "0, 0, 0"))
  (bind (_bblockinghit _binitialoverlap _time _distance _location _impactpoint _normal _impactnormal _physmat _hitactor _hitcomponent _hitbonename) (Collision|BreakHitResult ImpactResult))
  (bind _returnvalue (Class|ISFactory|CreateItem "/Game/Data/Inventory/Items/Generics/DA_Arrow.DA_Arrow"))
  (bind _outitemdropactor (Class|ItemBase|TryDrop _returnvalue (+ (Transformation|GetActorLocation) (* (Math|Vector|GetForwardVector (Transformation|GetActorRotation)) (Math|Random|RandomFloatinRange 15.0 3e+01))) (Transformation|GetActorRotation) true))
  (|CallParentFunction ImpactResult ImpactVelocity)
  (Class|KismetSystemLibrary|IsObjectOfSoftClass _hitactor "/Script/Engine.Pawn"
    (:True
      (Transformation|AttachComponentToComponent _outitemdropactor _hitcomponent _hitbonename "KeepWorld" "KeepWorld" "KeepRelative" true))))

(fn ConstructionScript)
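; BP_Stash is a stash actor in the chest system whose RPG inventory persists in the shared save game.
; On shared-save prep, the Saver component's event writes the inventory's item data into BP_EKSharedSave's StashInventory.
; On beginning with a loaded shared save, or completing a shared load, it wraps that data in a new RPGInventorySaveData and loads it back into the inventory.
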(event EventBeginPlay
  (|CallParentFunction) ; This node is disabled and will not be called.\nDrag off pins to build functionality.
)

(event Collision|EventActorBeginOverlap
  (params (OtherActor :type Actor%20Object%20Reference)))

(event EventTick
  (params (DeltaSeconds :type Float%20%28single-precision%29)))

(event OnBeginwithLoadedSharedSaveGame(Saver)
  (params (SharedSaveGame :type Default%20Save%20Game%20Object%20Reference))
  ;[1 0 0 0.5] Stash Inventory
  (bind _returnvalue (Game|ConstructObjectfromClass "/Script/RPGSystem.RPGInventorySaveData" (Variables|/Game/Data/SaveSystem/BP_EKSharedSave.BP_EKSharedSave_C|GetStashInventory (.AsBP%20EKShared%20Save (Utilities|Casting|CastToBP_EKSharedSave (Class|SSUtility|GetSharedSaveGame))))))
  (Class|InventoryBase|LoadSaveData (Variables|Default|GetRPGInventory) _returnvalue))

(event OnSharedLoadGameCompleted(Saver)
  (params (SlotName :type String) (UserIndex :type Integer) (SaveGameData :type Default%20Save%20Game%20Object%20Reference) (Instigator :type Object%20Object%20Reference))
  ;[1 0 0 0.5] Stash Inventory
  (bind _returnvalue (Game|ConstructObjectfromClass "/Script/RPGSystem.RPGInventorySaveData" (Variables|/Game/Data/SaveSystem/BP_EKSharedSave.BP_EKSharedSave_C|GetStashInventory (.AsBP%20EKShared%20Save (Utilities|Casting|CastToBP_EKSharedSave (Class|SSUtility|GetSharedSaveGame))))))
  (Class|InventoryBase|LoadSaveData (Variables|Default|GetRPGInventory) _returnvalue))

(event OnPrepSharedSave(Saver)
  (params (SaveGameData :type Default%20Save%20Game%20Object%20Reference) (SlotInfoItem :type Slot%20Info%20Item%20Object%20Reference) (Instigator :type Object%20Object%20Reference))
  ;[1 0 0 0.5] Stash Inventory
  (Variables|/Game/Data/SaveSystem/BP_EKSharedSave.BP_EKSharedSave_C|SetStashInventory (.AsBP%20EKShared%20Save (Utilities|Casting|CastToBP_EKSharedSave (Class|SSUtility|GetSharedSaveGame))) (Variables|/Script/RPGSystem.RPGInventorySaveData|GetRPGItemsSaveData (.AsRPGInventory%20Save%20Data (Utilities|Casting|CastToRPGInventorySaveData (Class|InventoryBase|CreateSaveData (Variables|Default|GetRPGInventory)))))))

(fn ConstructionScript
  (|CallParentFunction))
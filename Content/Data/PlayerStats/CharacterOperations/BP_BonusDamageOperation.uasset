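; BP_BonusDamageOperation is a character stat operation that derives bonus damage from a modifier value, apparently Strength.
; GetResultOperation takes the square root of ModifierValue, scales it by a fixed factor, rounds it and returns it as a double, giving diminishing returns as the stat grows.
; An unused math expression node holds the same formula written against STR.
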(fn GetResultOperation
  (return (Math|Conversions|ToFloat(Integer) (Math|Float|Round (* (Math|Float|Sqrt (Variables|Default|GetModifierValue)) 2.7)))))
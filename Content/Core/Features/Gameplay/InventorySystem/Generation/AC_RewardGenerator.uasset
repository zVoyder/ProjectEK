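; Actor component that fills its owner's RPG inventory with random gear, weapons, generic items and currency as rewards.
; BeginPlay caches the inventory; GenerateRewards, not called within this file, runs one generator per category.
; Gear, weapon and item generators roll counts and pick random map keys, with map values supplying generation data or amount ranges.
; Generic item count reuses WeaponsRange; currency is one ranged amount of CurrencyItem.
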(event EventBeginPlay
  (CallFunction|Init))

(event EventTick
  (params (DeltaSeconds :type Float%20%28single-precision%29)))

(fn GenerateRewards
  (Variables|Default|GetInventory
    (:then
      (CallFunction|GenerateGears)
      (CallFunction|GenerateWeapons)
      (CallFunction|GenerateItems)
      (CallFunction|GenerateCurrency))
    (:else)))

(fn Init
  (bind _output_get (Variables|Default|SetInventory (Actor|GetComponentbyClass (Components|GetOwner) "/Script/RPGSystem.RPGInventory")))
  (Utilities|IsValid _output_get
    (:Is%20Valid
      (Development|PrintString "RewardGenerator:Init: Inventory Not found." false true "(R=1.000000,G=0.000000,B=0.000000,A=1.000000)"))))

(fn GenerateGears
  (bind _gearsrange (Variables|Default|GetGearsRange))
  (bind _gears (Variables|Default|GetGears))
  (if (Utilities|Map|IsNotEmpty (Variables|Default|GetGears))
    (for _index (range 0 (- (Math|Random|RandomIntegerinRange (.value (.lowerbound _gearsrange)) (.value (.upperbound _gearsrange))) 1))
      (bind _keys (Utilities|Map|Keys _gears))
      (bind _returnvalue (Class|RPGFactory|CreateRPGGearItemwithGenerationSet (Utilities|Array|Get(acopy) _keys (Math|Random|RandomIntegerinRange 0 (- (Utilities|Map|Length _gears) 1))) (.Value (Utilities|Map|Find _gears (Utilities|Array|Get(acopy) _keys (Math|Random|RandomIntegerinRange 0 (- (Utilities|Map|Length _gears) 1)))))))
      (Class|InventoryBase|TryAddItem (Variables|Default|GetInventory) _returnvalue))))

(fn GenerateWeapons
  (bind _weapons (Variables|Default|GetWeapons))
  (bind _weaponsrange (Variables|Default|GetWeaponsRange))
  (if (Utilities|Map|IsNotEmpty (Variables|Default|GetWeapons))
    (for _index (range 0 (- (Math|Random|RandomIntegerinRange (.value (.lowerbound _weaponsrange)) (.value (.upperbound _weaponsrange))) 1))
      (bind _keys (Utilities|Map|Keys _weapons))
      (bind _returnvalue (Class|RPGFactory|CreateRPGGearItem (Utilities|Array|Get(acopy) _keys (Math|Random|RandomIntegerinRange 0 (- (Utilities|Map|Length _weapons) 1))) (.Value (Utilities|Map|Find _weapons (Utilities|Array|Get(acopy) _keys (Math|Random|RandomIntegerinRange 0 (- (Utilities|Map|Length _weapons) 1)))))))
      (Class|InventoryBase|TryAddItem (Variables|Default|GetInventory) _returnvalue))))

(fn GenerateItems
  (bind _generics (Variables|Default|GetGenerics))
  (bind _weaponsrange (Variables|Default|GetWeaponsRange))
  (if (Utilities|Map|IsNotEmpty (Variables|Default|GetGenerics))
    (for _index (range 0 (- (Math|Random|RandomIntegerinRange (.value (.lowerbound _weaponsrange)) (.value (.upperbound _weaponsrange))) 1))
      (bind _keys (Utilities|Map|Keys _generics))
      (Class|InventoryBase|AddNewItem (Variables|Default|GetInventory) (Utilities|Array|Get(acopy) _keys (Math|Random|RandomIntegerinRange 0 (- (Utilities|Map|Length _generics) 1))) (Math|Random|RandomIntegerinRange (.value (.lowerbound (.Value (Utilities|Map|Find _generics (Utilities|Array|Get(acopy) _keys (Math|Random|RandomIntegerinRange 0 (- (Utilities|Map|Length _generics) 1))))))) (.value (.upperbound (.Value (Utilities|Map|Find _generics (Utilities|Array|Get(acopy) _keys (Math|Random|RandomIntegerinRange 0 (- (Utilities|Map|Length _generics) 1))))))))))))

(fn GenerateCurrency
  (bind _currencyrange (Variables|Default|GetCurrencyRange))
  (Class|InventoryBase|AddNewItem (Variables|Default|GetInventory) (Variables|Default|GetCurrencyItem) (Math|Random|RandomIntegerinRange (.value (.lowerbound _currencyrange)) (.value (.upperbound _currencyrange)))))
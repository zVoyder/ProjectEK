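; Gameplay player state that tracks the player's health, initializes the levels manager and exposes the character stats component.
; The health resource attribute is fetched by tag at BeginPlay, and reaching its min or max triggers death or full-heal events.
; When AC_PlayerStats recalculates, max health updates from the MaxHealth stat a tick later.
; SaveGraph holds unconnected currency save and load logic that never runs.
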(event OnCalculatedFullStatsValues(AC_PlayerStats)
  (params (StatsBridge :type Stats%20Bridge%20Base%20Object%20Reference))
  (Utilities|FlowControl|DelayUntilNextTick)
  (Utilities|IsValid StatsBridge
    (:Is%20Valid
      (bind _healthattribute (Variables|Default|GetHealthAttribute)
        (:then
          (Class|ResourceAttribute|SetMaxValue _healthattribute (Class|StatsBridgeBase|GetFullStatValueasFloat StatsBridge "/Game/Data/PlayerStats/CoreStats/DA_MaxHealth.DA_MaxHealth")))
        (:else)))))

(event Custom|OnResourceAttributeReachedMinValue_Event
  (params (CurrentValue :type Float%20%28single-precision%29))
  (CallFunction|OnPlayerDeathEvent))

(event Custom|OnPlayerDeath_Event
  (Default|CallOnPlayerDeath)
  (Development|PrintString "Death"))

(event Custom|OnResourceAttributeReachedMaxValue_Event
  (params (CurrentValue :type Float%20%28single-precision%29))
  (CallFunction|OnPlayerFullHealedEvent))

(event Custom|OnPlayerFullHealed_Event
  (Default|CallOnPlayerFullHealed)
  (Development|PrintString "Full Heal"))

(event EventBeginPlay
  (bind _output_get (Variables|Default|SetHealthAttribute (Class|ResourceAttributesManager|GetAttributebyTag (Variables|Default|GetResourceAttributesManager) "(TagName=\"ResourceAttributes.Player.Health\")")))
  (EventDispatchers|AssignOnResourceAttributeReachedMinValue _output_get (delegate Custom|OnResourceAttributeReachedMinValue_Event))
  (EventDispatchers|AssignOnResourceAttributeReachedMaxValue _output_get (delegate Custom|OnResourceAttributeReachedMaxValue_Event))
  (Class|LevelsManager|Init (Variables|Default|GetLevelsManager)))

(fn ConstructionScript)

(fn GetCharacterStats
  (return (Variables|Default|GetAC_PlayerStats)))
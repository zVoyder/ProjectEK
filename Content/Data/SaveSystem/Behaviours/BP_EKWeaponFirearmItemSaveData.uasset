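; Save data behaviour for EKWeaponFirearmItem objects that persists a firearm's magazine state in the save system.
; SaveObjectData casts the object to a firearm item and stores its current magazine ammo and HasNewMag flag.
; LoadObjectData performs the same cast, then writes both saved values back through the ammo setter and the flag.
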(fn SaveObjectData
  (params (ObjectToSave :type Object%20Object%20Reference))
  (bind _asekweapon_firearm_item (Utilities|Casting|CastToEKWeaponFirearmItem ObjectToSave))
  (Variables|Default|SetSavedMagAmmo (Class|EKWeaponFirearmItem|GetCurrentMagAmmo _asekweapon_firearm_item))
  (Variables|Default|SetbSavedHasMag (Variables|/Script/ProjectEK.EKWeaponFirearmItem|GetbHasNewMag _asekweapon_firearm_item))
  (return true))

(fn LoadObjectData
  (params (ObjectToLoad :type Object%20Object%20Reference))
  (bind _asekweapon_firearm_item (Utilities|Casting|CastToEKWeaponFirearmItem ObjectToLoad))
  (Class|EKWeaponFirearmItem|SetCurrentMagAmmo _asekweapon_firearm_item (Variables|Default|GetSavedMagAmmo))
  (Variables|/Script/ProjectEK.EKWeaponFirearmItem|SetbHasNewMag _asekweapon_firearm_item (Variables|Default|GetbSavedHasMag))
  (return true))
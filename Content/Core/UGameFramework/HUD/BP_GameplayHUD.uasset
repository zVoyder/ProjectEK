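; Gameplay HUD that creates the main HUD widget and switches the crosshair based on what the player character's interactor highlights.
; On BeginPlay it adds WBP_GameplayHUD to the viewport, shows the default crosshair and binds to the BP_Interactor component's highlight and unhighlight dispatchers.
; Highlighting swaps in the pickup crosshair, and unhighlighting restores the default, so crosshair changes are event-driven without Tick.
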(event Custom|OnHighlight_Event
  (Class|CrosshairsUtility|SetCrosshairinViewport "/Game/Core/Features/UI/Crosshair/WBP_PickupCrosshair.WBP_PickupCrosshair_C" 0))

(event Custom|OnUnhighlight_Event
  (Class|CrosshairsUtility|SetDefaultCrosshairinViewport 0))

(event EventBeginPlay
  (bind _returnvalue (UserInterface|CreateWidget "/Game/Core/Features/UI/HUD/WBP_GameplayHUD.WBP_GameplayHUD_C" (Game|Player|GetOwningPlayerController)))
  (UserInterface|Viewport|AddtoViewport _returnvalue -1)
  (Variables|Default|SetWBP_GameplayHUD _returnvalue)
  (Class|CrosshairsUtility|SetDefaultCrosshairinViewport 0)
  (bind _output_get (Variables|Default|SetInteractor (Actor|GetComponentbyClass (Class|GameCastingHelper|GetGameCharacter) "/VUEDKCore/Systems/InteractSystem/Components/BP_Interactor.BP_Interactor_C")))
  (EventDispatchers|AssignOnHighlight _output_get (EventDispatchers|CreateEvent :!event Custom|OnHighlight_Event))
  (EventDispatchers|AssignOnUnhighlight _output_get (EventDispatchers|CreateEvent :!event Custom|OnUnhighlight_Event)))

(fn ConstructionScript)
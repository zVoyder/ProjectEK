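; Gear drop actor that represents an item in the world, can be highlighted, and is picked up on interaction.
; Pickup first tries equipping the item to an available slot without swapping, falls back to the player state's inventory, and destroys the actor only on success.
; Init gives the mesh the Pickup collision profile, and a SnapToGround helper traces downward to rest the actor's bounds on the hit surface.
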(event Custom|OnPickedUp)

(event EventHighlight
  (Default|Highlight (Variables|Default|GetAC_Highlighter)))

(event EventUnhighlight
  (Default|Unhighlight (Variables|Default|GetAC_Highlighter)))

(event EventOnInit
  (Collision|SetCollisionProfileName (Variables|Default|GetDropMesh) "Pickup" true :!class /Script/Engine.PrimitiveComponent))

(event EventInteract
  (CallFunction|Pickup))

(fn ConstructionScript)

(fn SnaptoGround
  (bind (_origin _boxextent) (Collision|GetActorBounds false false))
  (bind _returnvalue (Transformation|GetActorLocation))
  (bind (_outhit _returnvalue_2) (Collision|LineTraceByChannel _returnvalue (+ _returnvalue (* (Transformation|GetActorUpVector) 1e+07 -1.0)) "TraceTypeQuery1" false 0 "None"))
  (if _returnvalue_2
    (Transformation|SetActorLocation (Math|Vector|MakeVector (.X (Math|Vector|BreakVector (.ImpactPoint (Collision|BreakHitResult _outhit)))) (.Y (Math|Vector|BreakVector (.ImpactPoint (Collision|BreakHitResult _outhit)))) (+ (.Z (Math|Vector|BreakVector (.ImpactPoint (Collision|BreakHitResult _outhit)))) (- (.Z (Math|Vector|BreakVector _boxextent)) (- (.Z (Math|Vector|BreakVector _origin)) (.Z (Math|Vector|BreakVector (Transformation|GetActorLocation))))))) false true)))

(fn Pickup
  (bind _returnvalue (Class|GameCastingHelper|GetGameplayPlayerState))
  (bind _returnvalue_2 (Class|Equipment|TryEquipItemtoAvailableSlot (Variables|/Script/ProjectEK.GameplayPlayerState|GetEquipment _returnvalue) (Variables|Default|GetRelatedItem) 0 false true))
  (if _returnvalue_2
    (CallFunction|OnPickedUp :!label _label)
    (Actor|DestroyActor)
    (else
      (bind _returnvalue_3 (Class|InventoryBase|TryAddItem (Variables|/Script/ProjectEK.GameplayPlayerState|GetInventory _returnvalue) (Variables|Default|GetRelatedItem)))
      (if _returnvalue_3
        (goto _label)))))

(fn CanbeInteracted
  (return true))

(fn GetHUDInteractionInfo
  (return "0, 0, 0" "" 0))
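; BP_Chest is an interactable chest that opens a loot panel showing its inventory through the gameplay controller.
; On interaction it plays an open montage and fires overridable hooks for opening and first-time opening.
; It listens to the menu manager, and closing the Character menu while open triggers the close hook and montage.
; KeepOpen makes the chest animate open only the first time and never animate closed.
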(event Custom|OnMenuClosed_Event
  (params (MenuWidget :type Menu%20Widget%20Object%20Reference) (MenuTag :type Gameplay%20Tag%20Structure))
  (if (and (== MenuTag "(TagName=\"UI.Menu.Character\")") (Variables|Default|GetbIsOpen))
    (Variables|Default|SetbIsOpen false)
    (CallFunction|ManageCloseMontage)
    (CallFunction|OnChestClosed)))

(event Custom|OnChestOpened)

(event Custom|OnChestClosed)

(event Custom|OnChestFirstOpen)

(event Custom|ManageOpenMontage
  (if (Variables|Montages|GetbKeepOpen)
    (if (not (Variables|Default|GetbHasBeenEverOpened))
      (Animation|Montage|PlayMontage (Variables|Default|GetSkeletalMesh) (Variables|Montages|GetOpenMontage) :!label _label))
    (else
      (goto _label))))

(event Custom|ManageCloseMontage
  (if (not (Variables|Montages|GetbKeepOpen))
    (Animation|Montage|PlayMontage (Variables|Default|GetSkeletalMesh) (Variables|Montages|GetCloseMontage))))

(event EventInteract
  (Default|OpenLootPanel (Variables|Default|GetBPGameplayController) (Variables|Default|GetRPGInventory) (Variables|Default|GetChestName))
  (Variables|Default|SetbIsOpen true)
  (CallFunction|ManageOpenMontage)
  (CallFunction|OnChestOpened)
  (if (not (Variables|Default|GetbHasBeenEverOpened))
    (CallFunction|OnChestFirstOpen)
    (Variables|Default|SetbHasBeenEverOpened true)))

(event EventBeginPlay
  (bind _asbp_gameplay_controller (Utilities|Casting|CastToBP_GameplayController (Class|GameCastingHelper|GetGameplayController)))
  (bind _output_get (Variables|Default|SetBPGameplayController _asbp_gameplay_controller))
  (EventDispatchers|AssignOnMenuClosed (Variables|/Script/ProjectEK.ProjectEKPlayerController|GetMenuManager _output_get) (EventDispatchers|CreateEvent :!event Custom|OnMenuClosed_Event)))

(fn ConstructionScript
  (|CallParentFunction))